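; Base Blueprint for economy buildings that handles their world-space health bar widget.
; Each tick it rotates the Widget component from the building's location toward a point 200 units behind the player pawn, approximating a camera-facing billboard.
; The SetupHealthBar event casts the widget's user object to BuildingHealthBar and passes the building in as its owner.
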(event EventTick
  (params (DeltaSeconds :type Float%20%28single-precision%29))
  (bind _returnvalue (Game|Player|GetPlayerPawn 0))
  (Transformation|SetWorldRotation (Variables|Default|GetWidget) (Math|Rotator|FindLookatRotation (Transformation|GetActorLocation) (- (Transformation|GetActorLocation _returnvalue) (* (Math|Vector|GetForwardVector (Transformation|GetActorRotation _returnvalue)) 2e+02))) false false))

(event EventSetupHealthBar
  (bind _asbuilding_health_bar (Utilities|Casting|CastToBuildingHealthBar (UserInterface|GetUserWidgetObject (Variables|Default|GetWidget))))
  (Default|SetOwningBuilding _asbuilding_health_bar self))

(fn ConstructionScript)