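; BaseUnitBP is a base unit Blueprint that manages an overhead-style health bar widget for its unit.
; Each tick it rotates the HealthBar component from the unit's location toward a point behind the first player's pawn, billboard-style, using a fixed offset along that pawn's forward vector.
; The SetupHealthBar event casts the component's widget to UnitHealthBar and passes the unit in as its owner.
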(event EventSetupHealthBar
  (bind _asunit_health_bar (Utilities|Casting|CastToUnitHealthBar (UserInterface|GetUserWidgetObject (Variables|Default|GetHealthBar))))
  (Default|SetOwningUnit _asunit_health_bar self))

(event EventTick
  (params (DeltaSeconds :type Float%20%28single-precision%29))
  (bind _returnvalue (Game|Player|GetPlayerPawn 0))
  (Transformation|SetWorldRotation (Variables|Default|GetHealthBar) (Math|Rotator|FindLookatRotation (Transformation|GetActorLocation) (- (Transformation|GetActorLocation _returnvalue) (* (Math|Vector|GetForwardVector (Transformation|GetActorRotation _returnvalue)) 2e+02))) false false))

(fn ConstructionScript)